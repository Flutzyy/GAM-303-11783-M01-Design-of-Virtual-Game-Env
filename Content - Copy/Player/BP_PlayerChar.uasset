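; BP_PlayerChar is the player character, with Enhanced Input look, movement, jump, sprint and interaction.
; Interact either drops the held object or line-traces from the camera and sends an interface message, passing itself, to the hit actor.
; Sprint press and release share a FlipFlop that switches walk speed, acting as hold-to-sprint.
; It also tracks and prints score and health, quitting the game when health falls below zero.
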(event `EnhancedInput|/Game/Inputs/Input_Look`
  (params (ActionValue :type "Vector2D Structure") (ElapsedSeconds :type "Float (double-precision)") (TriggeredSeconds :type "Float (double-precision)") (InputAction :type "InputAction Object Reference" :default "/Game/Inputs/Input_Look.Input_Look"))
  ;[1 1 1] Player Controls
  (:`Triggered`
    (`self.AddControllerYawInput` ActionValue_X)
    (`self.AddControllerPitchInput` ActionValue_Y)))

(event `EnhancedInput|/Game/Inputs/Input_Movement`
  (params (ActionValue :type "Vector2D Structure") (ElapsedSeconds :type "Float (double-precision)") (TriggeredSeconds :type "Float (double-precision)") (InputAction :type "InputAction Object Reference" :default "/Game/Inputs/Input_Movement.Input_Movement"))
  (bind (_returnvalue_roll _returnvalue_pitch _returnvalue_yaw) (`KismetMathLibrary.BreakRotator` (`self.GetControlRotation`)))
  ;[1 1 1] Player Controls
  (:`Triggered`
    (`self.AddMovementInput` (`KismetMathLibrary.GetRightVector` (`KismetMathLibrary.MakeRotator` _returnvalue_roll 0.0 _returnvalue_yaw)) ActionValue_X)
    (`self.AddMovementInput` (`KismetMathLibrary.GetForwardVector` (`KismetMathLibrary.MakeRotator` 0.0 0.0 _returnvalue_yaw)) ActionValue_Y)))

(event `EnhancedInput|/Game/Inputs/Input_Jump`
  (params (ActionValue :type Boolean) (ElapsedSeconds :type "Float (double-precision)") (TriggeredSeconds :type "Float (double-precision)") (InputAction :type "InputAction Object Reference" :default "/Game/Inputs/Input_Jump.Input_Jump"))
  ;[1 1 1] Player Controls
  (:`Started`
    (`self.Jump`))
  (:`Canceled`
    (`self.StopJumping`)))

(event `EnhancedInput|/Game/Inputs/Input_Interact`
  (params (ActionValue :type Boolean) (ElapsedSeconds :type "Float (double-precision)") (TriggeredSeconds :type "Float (double-precision)") (InputAction :type "InputAction Object Reference" :default "/Game/Inputs/Input_Interact.Input_Interact"))
  (bind _camera (`self.Camera`))
  (bind _returnvalue (`SceneComponent.K2_GetComponentLocation` _camera))
  ;[1 1 1] Player Controls
  (:`Started`
    (if (`self.IsHolding`)
      (message `/Game/Interfaces/Interface_Interact.INT_Drop` (`self.HitObject`))
      (set `self.IsHolding` false)
      (else
        (bind _outhit (`KismetSystemLibrary.LineTraceSingle` :`Start` _returnvalue :`End` (+ _returnvalue (* (`SceneComponent.GetForwardVector` _camera) 800.0)) :`TraceChannel` "TraceTypeQuery1" :`DrawDebugType` "ForDuration"))
        (if true
          (bind (_bblockinghit _binitialoverlap _time _distance _location _impactpoint _normal _impactnormal _physmat _hitactor) (`GameplayStatics.BreakHitResult` _outhit))
          (set `self.HitObject` _hitactor)
          (message `/Game/Interfaces/Interface_Interact.INT_Interact` _hitactor self))))))

(event `AddScore`
  (params (AddAmount :type Integer))
  ;[1 1 1] Player Controls
  (bind _output_get (set `self.Score` (+ (`self.Score`) AddAmount)))
  (`KismetSystemLibrary.PrintString` (`KismetStringLibrary.Conv_IntToString` _output_get)))

(event `self.ReceiveAnyDamage`
  (params (Damage :type "Float (single-precision)") (DamageType :type "DamageType Object Reference") (InstigatedBy :type "Controller Object Reference") (DamageCauser :type "Actor Object Reference"))
  ;[1 1 1] Player Controls
  (bind _output_get (set `self.Health` (- (`self.Health`) Damage)))
  (`KismetSystemLibrary.PrintString` (`KismetStringLibrary.Conv_DoubleToString` _output_get))
  (if (< (`self.Health`) 0.0)
    (`KismetSystemLibrary.QuitGame` null "Quit")))

(event `DropObject`
  ;[1 1 1] Player Controls
)

(event `InputAction|Sprint`
  (params (Key :type "Key Structure"))
  (bind _charactermovement (`self.CharacterMovement`))
  ;[1 1 1] Sprinting
  (:`Pressed`
    (`/Engine/EditorBlueprintResources/StandardMacros.FlipFlop` :!label _label
      (:`A`
        (set `CharacterMovementComponent.MaxWalkSpeed` 1000.0 _charactermovement)
        (set `self.IsSprinting` true))
      (:`B`
        (set `CharacterMovementComponent.MaxWalkSpeed` 600.0 _charactermovement)
        (set `self.IsSprinting` false))))
  (:`Released`
    (goto _label)))

(fn `UserConstructionScript`)